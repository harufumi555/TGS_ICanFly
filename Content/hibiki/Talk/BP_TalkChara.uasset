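; BP_TalkChara is a talking-character Blueprint that shows paged dialogue in a WBP_MessageWindow widget.
; Talk opens the window and Talkread advances it, each using TalkNum to pick one of five DataTables.
; Pages load speaker and message by sequentially numbered row names, and the window closes and resets to page one after the last.
; The last page is counted only from DT_TalkData at BeginPlay and applies to every table.
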(event Custom|Talk
  (params (TalkNum :type Integer))
  (switch int TalkNum
    (:0
      (CallFunction|NewFunction "/Game/hibiki/Talk/Talkdata/DT_TalkData.DT_TalkData"))
    (:1
      (CallFunction|NewFunction "/Game/hibiki/Talk/Talkdata/DT_TalkData_2.DT_TalkData_2"))
    (:2
      (CallFunction|NewFunction "/Game/hibiki/Talk/Talkdata/DT_TalkData_4.DT_TalkData_4"))
    (:3
      (CallFunction|NewFunction "/Game/hibiki/Talk/Talkdata/DT_TalkData_3.DT_TalkData_3"))
    (:4
      (CallFunction|NewFunction "/Game/hibiki/Talk/Talkdata/DT_TalkData_5.DT_TalkData_5"))))

(event Custom|Talkread
  (switch int (stale Custom|Talk TalkNum)
    (:0
      (CallFunction|ShowNextPage "/Game/hibiki/Talk/Talkdata/DT_TalkData.DT_TalkData"))
    (:1
      (CallFunction|ShowNextPage "/Game/hibiki/Talk/Talkdata/DT_TalkData_2.DT_TalkData_2"))
    (:2
      (CallFunction|ShowNextPage "/Game/hibiki/Talk/Talkdata/DT_TalkData_4.DT_TalkData_4"))
    (:3
      (CallFunction|ShowNextPage "/Game/hibiki/Talk/Talkdata/DT_TalkData_3.DT_TalkData_3"))
    (:4
      (CallFunction|ShowNextPage "/Game/hibiki/Talk/Talkdata/DT_TalkData_5.DT_TalkData_5"))))

(event EventBeginPlay
  (bind _returnvalue (UserInterface|CreateWidget "/Game/hibiki/Talk/WBP_MessageWindow.WBP_MessageWindow_C"))
  (Variables|Default|SetMessageWindow _returnvalue)
  (CallFunction|CheckLastPage "/Game/hibiki/Talk/Talkdata/DT_TalkData.DT_TalkData") ; 会話ページの番号を取得
)

(fn ConstructionScript)

(fn CheckLastPage
  (params (Table :type Data%20Table%20Object%20Reference))
  (bind _outrownames (DataTable|GetDataTableRowNames Table))
  (for _array_element _outrownames
    (Math|Integer|IncrementInt (Variables|Default|GetLastPage))))

(fn LoadTalkData
  (params (DataTable :type Data%20Table%20Object%20Reference))
  (bind _returnvalue (Utilities|GetDataTableRow DataTable (Utilities|String|StringToName (Utilities|String|ToString(Integer) (Variables|Default|GetCurrentPage)))) ; データテーブルの値を見る（その際、名前は連番のため[1.２．３]になる）
    (:then
      (Default|SetTalkMessage (Variables|Default|GetMessageWindow) (.Talker (Utilities|Struct|BreakSTR_Talkinfo _returnvalue)) (.TalkMessage (Utilities|Struct|BreakSTR_Talkinfo _returnvalue))))))

(fn ShowNextPage
  (params (DataTable :type Data%20Table%20Object%20Reference))
  (if (Variables|Default|Getis_ShawMessage) ; widgetが表示されているかどうか
    (Math|Integer|IncrementInt (Variables|Default|GetCurrentPage)
      (:%20%20
        (if (> (Variables|Default|GetCurrentPage) (Variables|Default|GetLastPage)) ; ページ数がラストをこえたかどうか
          (Variables|Default|SetCurrentPage 1) ; 初めのページに戻す
          (Variables|Default|Setis_ShawMessage false)
          (Widget|RemovefromParent (Variables|Default|GetMessageWindow)) ; widgetを閉じる
          (else
            (CallFunction|LoadTalkData DataTable)))))))

(fn NewFunction
  (params (DataTable :type Data%20Table%20Object%20Reference))
  (if (not (Variables|Default|Getis_ShawMessage))
    (Variables|Default|Setis_ShawMessage true)
    (CallFunction|LoadTalkData DataTable)
    (UserInterface|Viewport|AddtoViewport (Variables|Default|GetMessageWindow) 0)))